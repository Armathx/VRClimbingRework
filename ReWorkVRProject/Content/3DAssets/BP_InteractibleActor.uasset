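; BP_InteractibleActor is a skeletal mesh actor that a motion-controller hand can grab by individual bones.
; On grab, the hand mesh attaches to the bone; for non-pelvis bones, physics simulates below it and a timer-driven PhysicsHandle follows the controller.
; On drop, the hand returns to its controller while a timeline drives physics blend weight before simulation stops.
; Actor overlap applies physical animation settings from the pelvis down.
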(event `self.ReceiveActorBeginOverlap`
  (params (OtherActor :type "Actor Object Reference"))
  (`PhysicalAnimationComponent.SetSkeletalMeshComponent` (`self.PhysicalAnimation`) (`self.SkeletalMesh`))
  (`PhysicalAnimationComponent.ApplyPhysicalAnimationSettingsBelow` (`self.PhysicalAnimation`) "pelvis" (make `PhysicalAnimationData` true 1000.0 100.0 100.0 100.0) true))

(event `self.GrabComponent.OnGrabbed`
  (params (`Self Reference` :type "/Game/VRTemplate/Blueprints/GrabComponent Object Reference") (BoneName :type Name) (HandMesh :type "SkeletalMeshComponent Object Reference") (PhysicsHandle :type "PhysicsHandleComponent Object Reference") (MotionController :type "MotionControllerComponent Object Reference"))
  (bind _grabbedbone (`self.GrabbedBone`))
  (bind _skeletalmesh (`self.SkeletalMesh`))
  (bind _grabbedbone_2 (`self.GrabbedBone`))
  (set `self.MotionController` MotionController)
  (set `self.GrabbedBone` BoneName)
  (bind _output_get (set `self.HandMesh` HandMesh))
  (set `self.PhysicsHandle` PhysicsHandle)
  (set `self.RelativeTransformBeforeGrab` (`SceneComponent.GetRelativeTransform` _output_get))
  (`SceneComponent.K2_AttachToComponent` _output_get (`self.SkeletalMesh`) _grabbedbone "KeepWorld" "KeepWorld" "KeepWorld" true)
  (if (!= _grabbedbone "pelvis")
    (`|ExecutionSequence`
      (:`then_0`
        (`SkeletalMeshComponent.SetAllBodiesBelowSimulatePhysics` _skeletalmesh _grabbedbone_2 true true))
      (:`then_1`
        (`SkeletalMeshComponent.SetAllBodiesBelowPhysicsBlendWeight` _skeletalmesh _grabbedbone_2 1.0 false true)
        (`PhysicsHandleComponent.GrabComponentAtLocation` (`self.PhysicsHandle`) (`self.SkeletalMesh`) (`self.GrabbedBone`) (`SceneComponent.K2_GetComponentLocation` (`self.MotionController`)))
        (bind _returnvalue (`KismetSystemLibrary.K2_SetTimerDelegate` (delegate `MakePhysicsHandleFollowMotionController`) 0.01 true))
        (set `self.Timer` _returnvalue)))))

(event `MakePhysicsHandleFollowMotionController`
  (`PhysicsHandleComponent.SetTargetLocation` (`self.PhysicsHandle`) (`SceneComponent.K2_GetComponentLocation` (`self.MotionController`))))

(event `self.GrabComponent.OnDropped`
  (params (`Self Reference` :type "/Game/VRTemplate/Blueprints/GrabComponent Object Reference"))
  (bind (_relativetransformbeforegrab_location _relativetransformbeforegrab_rotation) (`KismetMathLibrary.BreakTransform` (`self.RelativeTransformBeforeGrab`)))
  (bind _grabbedbone (`self.GrabbedBone`))
  (bind _skeletalmesh (`self.SkeletalMesh`))
  (`KismetSystemLibrary.K2_ClearAndInvalidateTimerHandle` (`self.Timer`))
  (`SceneComponent.K2_AttachToComponent` (`self.HandMesh`) (`self.MotionController`) "None" "KeepWorld" "KeepWorld" "KeepWorld" true)
  (`|ExecutionSequence`
    (:`then_0`
      (`KismetSystemLibrary.MoveComponentTo` (`self.HandMesh`) _relativetransformbeforegrab_location _relativetransformbeforegrab_rotation)
      (`PhysicsHandleComponent.ReleaseComponent` (`self.PhysicsHandle`)))
    (:`then_1`
      (bind (_direction _blend) (`Timeline|Timeline` :!via `PlayFromStart`)
        (:`Update`
          (`SkeletalMeshComponent.SetAllBodiesBelowPhysicsBlendWeight` _skeletalmesh _grabbedbone _blend false true))
        (:`Finished`
          (`SkeletalMeshComponent.SetAllBodiesBelowSimulatePhysics` _skeletalmesh _grabbedbone false true))))))

(fn `UserConstructionScript`)