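; BP_ClimbableStoneHard is a moving mossy stone, apparently a harder grabbable hold for climbing.
; On BeginPlay it caches the mesh's world location and starts the MoveGrabbable timeline.
; Each update moves the actor along the mesh's right vector by the timeline's Offset scaled by OffsetValue, relative to that start point, without sweeping.
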(event `self.ReceiveBeginPlay`
  (bind _output_get (set `self.InitialLocation` (`SceneComponent.K2_GetComponentLocation` (`self.Mossy_Stone_sdAfk_Mid`))))
  (bind (_direction _offset) (`Timeline|MoveGrabbable` :!via `PlayFromStart`)
    (:`Update`
      (`self.K2_SetActorLocation` (+ (* (* _offset (`SceneComponent.GetRightVector` (`self.Mossy_Stone_sdAfk_Mid`))) (`self.OffsetValue`)) _output_get)))))

(fn `UserConstructionScript`)